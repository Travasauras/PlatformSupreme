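; BP_TurretMobile is a moving turret enemy that shoots at the player and can be destroyed through contact with its head.
; On BeginPlay, a timeline lerps it along world X from its spawn point.
; Box overlap by the player starts looping timers that periodically snap the pivot toward them and spawn projectiles, cleared on exit.
; Player overlap with HeadBox gives a small upward launch and destroys the turret.
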(event `self.ReceiveBeginPlay`
  (bind _output_get (set `self.startv` (`self.K2_GetActorLocation`)))
  (set `self.endv` (+ _output_get (`KismetMathLibrary.MakeVector` 500.0)))
  (bind (_direction _alpha) (`Timeline|Timeline` :!via `PlayFromStart`)
    (:`Update`
      (`self.K2_SetActorLocation` (`KismetMathLibrary.VLerp` (`self.startv`) (`self.endv`) _alpha)))))

(event `FireAtPlayer`
  (`|SpawnActorFromClass` "/Game/Enemies/Turret/BP_TurretProjectile.BP_TurretProjectile_C" (`SceneComponent.K2_GetComponentToWorld` (`self.ProjectileSpawn`)) "Undefined" "MultiplyWithRoot" null null))

(event `FollowPlayer`
  (`SceneComponent.K2_SetWorldRotation` (`self.pivot`) (`KismetMathLibrary.FindLookAtRotation` (`self.K2_GetActorLocation`) (`self.K2_GetActorLocation` (`GameplayStatics.GetPlayerCharacter` 0))) false false))

(event `self.box_0.OnComponentBeginOverlap`
  (params (OverlappedComponent :type "PrimitiveComponent Object Reference") (OtherActor :type "Actor Object Reference") (OtherComp :type "PrimitiveComponent Object Reference") (OtherBodyIndex :type Integer) (bFromSweep :type Boolean) (SweepResult :type "HitResult Structure (by ref)"))
  (cast `/Game/Player/BP_PlayerChar` OtherActor)
  (`KismetSystemLibrary.K2_SetTimer` null "FollowPlayer" 0.5 true)
  (`KismetSystemLibrary.K2_SetTimer` null "FireAtPlayer" 1.0 true))

(event `self.box_0.OnComponentEndOverlap`
  (params (OverlappedComponent :type "PrimitiveComponent Object Reference") (OtherActor :type "Actor Object Reference") (OtherComp :type "PrimitiveComponent Object Reference") (OtherBodyIndex :type Integer))
  (cast `/Game/Player/BP_PlayerChar` OtherActor)
  (`KismetSystemLibrary.K2_ClearTimer` null "FollowPlayer")
  (`KismetSystemLibrary.K2_ClearTimer` null "FireAtPlayer"))

(event `self.HeadBox.OnComponentBeginOverlap`
  (params (OverlappedComponent :type "PrimitiveComponent Object Reference") (OtherActor :type "Actor Object Reference") (OtherComp :type "PrimitiveComponent Object Reference") (OtherBodyIndex :type Integer) (bFromSweep :type Boolean) (SweepResult :type "HitResult Structure (by ref)"))
  (bind _asbp_player_char (cast `/Game/Player/BP_PlayerChar` OtherActor))
  (`Character.LaunchCharacter` _asbp_player_char (0.0 0.0 10.0) false false)
  (`self.K2_DestroyActor`))

(fn `UserConstructionScript`)