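; Enemy turret that aims and fires at the player while they are inside its Box_0 trigger.
; Overlap by BP_PlayerChar starts two looping timers by function name, and leaving the box clears both.
; FollowPlayer periodically snaps Pivot toward player character 0 instead of updating on Tick.
; FireAtPlayer spawns BP_TurretProjectile at the ProjectileSpawn transform on its own, slower interval.
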(event `FireAtPlayer`
  (`|SpawnActorFromClass` "/Game/Enemies/Turret/BP_TurretProjectile.BP_TurretProjectile_C" (`SceneComponent.K2_GetComponentToWorld` (`self.ProjectileSpawn`)) "Undefined" "MultiplyWithRoot" null null))

(event `FollowPlayer`
  (`SceneComponent.K2_SetWorldRotation` (`self.pivot`) (`KismetMathLibrary.FindLookAtRotation` (`self.K2_GetActorLocation`) (`self.K2_GetActorLocation` (`GameplayStatics.GetPlayerCharacter` 0))) false false))

(event `self.box_0.OnComponentBeginOverlap`
  (params (OverlappedComponent :type "PrimitiveComponent Object Reference") (OtherActor :type "Actor Object Reference") (OtherComp :type "PrimitiveComponent Object Reference") (OtherBodyIndex :type Integer) (bFromSweep :type Boolean) (SweepResult :type "HitResult Structure (by ref)"))
  (cast `/Game/Player/BP_PlayerChar` OtherActor)
  (`KismetSystemLibrary.K2_SetTimer` null "FollowPlayer" 0.5 true)
  (`KismetSystemLibrary.K2_SetTimer` null "FireAtPlayer" 1.0 true))

(event `self.box_0.OnComponentEndOverlap`
  (params (OverlappedComponent :type "PrimitiveComponent Object Reference") (OtherActor :type "Actor Object Reference") (OtherComp :type "PrimitiveComponent Object Reference") (OtherBodyIndex :type Integer))
  (cast `/Game/Player/BP_PlayerChar` OtherActor)
  (`KismetSystemLibrary.K2_ClearTimer` null "FollowPlayer")
  (`KismetSystemLibrary.K2_ClearTimer` null "FireAtPlayer"))

(fn `UserConstructionScript`)