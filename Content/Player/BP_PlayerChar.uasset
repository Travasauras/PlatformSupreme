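; Player character for a side-scrolling game, moving along the X axis with sprint, variable-height jump, interaction and projectile fire.
; Interact sphere-traces in the facing direction and messages the hit actor to pick up or drop; fire spawns BP_Projectile after a short timer.
; It creates the HUD widget and pushes health, score and timer start to it.
; Zero health calls Die, which calls a still-empty Respawn function.
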(event `self.ReceiveBeginPlay`
  ; Widget
  (set `self.CurrentHealth` (`self.MaxHealth`))
  (bind _returnvalue (`|CreateWidget` "/Game/Player/Player_Widget.Player_Widget_C" (`GameplayStatics.GetPlayerController` 0)))
  (bind _output_get (set `self.HUDref` _returnvalue))
  (`UserWidget.AddToViewport` _returnvalue 0)
  (`UserWidget.AddToViewport` _output_get 0)
  (`/Game/Player/Player_Widget.updateHP` _output_get (`self.CurrentHealth`) (`self.MaxHealth`)))

(event `EnhancedInput|/Game/inputs/input_jump`
  (params (ActionValue :type Boolean) (ElapsedSeconds :type "Float (double-precision)") (TriggeredSeconds :type "Float (double-precision)") (InputAction :type "InputAction Object Reference" :default "/Game/inputs/input_jump.input_jump"))
  (bind (_returnvalue_x _returnvalue_y _returnvalue_z) (`KismetMathLibrary.BreakVector` (`self.GetVelocity`)))
  ; VariableJump
  (:`Started`
    (`self.Jump`))
  (:`Completed`
    (if (> _returnvalue_z 0.0)
      (`self.LaunchCharacter` (`KismetMathLibrary.MakeVector` 0.0 0.0 (* _returnvalue_z 0.65)) false true))))

(event `EnhancedInput|/Game/inputs/input_movement`
  (params (ActionValue :type "Vector2D Structure") (ElapsedSeconds :type "Float (double-precision)") (TriggeredSeconds :type "Float (double-precision)") (InputAction :type "InputAction Object Reference" :default "/Game/inputs/input_movement.input_movement"))
  ; Movement and timer start
  (:`Triggered`
    (`|ExecutionSequence`
      (:`then_0`
        (`self.AddMovementInput` (1.0 0.0 0.0) ActionValue_X))
      (:`then_1`
        (if (not (`self.HasTimerStarted?`))
          (`/Game/Player/Player_Widget.StartTimer` (`self.HUDref`))
          (if (> ActionValue_X 0.0)
            (set `self.FacingDirection` 1.0)
            (`SceneComponent.K2_SetRelativeRotation` :`self` (`self.Cylinder`))
            (elif (< ActionValue_X 0.0)
              (set `self.FacingDirection` -1.0)
              (`SceneComponent.K2_SetRelativeRotation` (`self.Cylinder`) (struct :`Pitch` 180.0) false false))))))))

(event `EnhancedInput|/Game/inputs/input_interact`
  (params (ActionValue :type Boolean) (ElapsedSeconds :type "Float (double-precision)") (TriggeredSeconds :type "Float (double-precision)") (InputAction :type "InputAction Object Reference" :default "/Game/inputs/input_interact.input_interact"))
  (bind _returnvalue (`self.K2_GetActorLocation`))
  ; Interact
  (:`Started`
    (if (`self.isHolding?`)
      (message `/Game/interface/Interface_interact.Int_drop` (`self.HitObject`))
      (set `self.isHolding?` false)
      (else
        (bind (_outhit _returnvalue_2) (`KismetSystemLibrary.SphereTraceSingle` :`Start` _returnvalue :`End` (+ (`KismetMathLibrary.MakeVector` (* (`self.FacingDirection`) 100.0)) _returnvalue) :`Radius` 100.0 :`TraceChannel` "TraceTypeQuery1" :`DrawDebugType` "ForDuration"))
        (if _returnvalue_2
          (bind (_bblockinghit _binitialoverlap _time _distance _location _impactpoint _normal _impactnormal _physmat _hitactor) (`GameplayStatics.BreakHitResult` _outhit))
          (set `self.HitObject` _hitactor)
          (message `/Game/interface/Interface_interact.INT_interact` _hitactor self))))))

(event `EnhancedInput|/Game/inputs/input_fire`
  (params (ActionValue :type Boolean) (ElapsedSeconds :type "Float (double-precision)") (TriggeredSeconds :type "Float (double-precision)") (InputAction :type "InputAction Object Reference" :default "/Game/inputs/input_fire.input_fire"))
  ; fire
  ;; fire
  (:`Started`
    (`KismetSystemLibrary.K2_SetTimer` null "FireEvent" 0.15)))

(event `FireEvent`
  ; fire
  ;; fire
  (bind _returnvalue (`|SpawnActorFromClass` "/Game/Player/BP_Projectile.BP_Projectile_C" (`SceneComponent.K2_GetComponentToWorld` (`self.Arrow1`)) "Undefined" "MultiplyWithRoot" self null))
  (`/Engine/EditorBlueprintResources/StandardMacros.IsValid` _returnvalue))

(event `addScore`
  (params (AddAmount :type Integer))
  ; AddScore
  (bind _output_get (set `self.score` (+ (`self.score`) AddAmount)))
  (`/Game/Player/Player_Widget.AddScore` (`self.HUDref`) "" _output_get))

(event `EnhancedInput|/Game/inputs/input_sprint`
  (params (ActionValue :type Boolean) (ElapsedSeconds :type "Float (double-precision)") (TriggeredSeconds :type "Float (double-precision)") (InputAction :type "InputAction Object Reference" :default "/Game/inputs/input_sprint.input_sprint"))
  ; Sprint
  (:`Started`
    (set `CharacterMovementComponent.MaxWalkSpeed` 900.0 (`self.CharacterMovement`)))
  (:`Completed`
    (set `CharacterMovementComponent.MaxWalkSpeed` 500.0 (`self.CharacterMovement`))))

(event `CheckHealth`
  ; Health and damage
  (if (<= (`self.CurrentHealth`) 0.0)
    (`self.Die`)))

(event `self.ReceiveAnyDamage`
  (params (Damage :type "Float (single-precision)") (DamageType :type "DamageType Object Reference") (InstigatedBy :type "Controller Object Reference") (DamageCauser :type "Actor Object Reference"))
  ; Health and damage
  (set `self.DamageCauser` DamageCauser)
  (set `self.CurrentHealth` (- (`self.CurrentHealth`) Damage))
  (`self.CheckHealth`)
  (`/Game/Player/Player_Widget.updateHP` (`self.HUDref`) (`self.CurrentHealth`) (`self.MaxHealth`)))

(event `HealthBonus`
  (params (MAXHealth :type "Float (double-precision)"))
  ; Health and damage
  (bind _output_get (set `self.MAXHealth` MAXHealth))
  (set `self.CurrentHealth` _output_get)
  (`/Game/Player/Player_Widget.updateHP` (`self.HUDref`) (`self.CurrentHealth`) (`self.MaxHealth`)))

(event `Die`
  ; Health and damage
  (`self.Respawn`))

(event `RefreshHealth`
  ; Health and damage
  (`/Engine/EditorBlueprintResources/StandardMacros.IsValid` (`self.HUDref`)
    (:`Is Valid`
      (`/Game/Player/Player_Widget.updateHP` (`self.HUDref`) (`self.CurrentHealth`) (`self.MaxHealth`)))))

(event `playerDeath`)

(fn `CheckHP`)

(fn `Respawn`)

(fn `UserConstructionScript`)